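; Paper2D side-scrolling player character with Enhanced Input movement, jumping, two attacks and a roll.
; Tick picks idle, run, jump or fall flipbooks from velocity and damages every actor overlapping the Hitbox.
; Attacks and rolls play one-shot flipbooks behind animation, movement and turning lock flags, which clear when playback finishes.
; The roll applies curve-scaled root motion along the facing direction, gated by a DoOnce that resets after a delay.
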(event OnFinishedPlaying(Sprite)
  (CallFunction|RestartAnimation))

(event Input|EnhancedActionEvents|EnhancedInputActionIA_Jump
  (params (ActionValue :type Boolean) (ElapsedSeconds :type Float%20%28double-precision%29) (TriggeredSeconds :type Float%20%28double-precision%29) (InputAction :type Input%20Action%20Object%20Reference :default "/Game/Input/Actions/IA_Jump.IA_Jump"))
  (bind _isunmovableanimation (Variables|Default|GetIsUnmovableAnimation))
  (:Started
    (if (not _isunmovableanimation)
      (Character|Jump)))
  (:Canceled
    (if (not _isunmovableanimation)
      (Character|StopJumping))))

(event Input|EnhancedActionEvents|EnhancedInputActionIA_Move
  (params (ActionValue :type Float%20%28double-precision%29) (ElapsedSeconds :type Float%20%28double-precision%29) (TriggeredSeconds :type Float%20%28double-precision%29) (InputAction :type Input%20Action%20Object%20Reference :default "/Game/Input/Actions/IA_Move.IA_Move"))
  (if (not (Variables|Default|GetIsUnmovableAnimation))
    (Pawn|Input|AddMovementInput "1.000000,0.000000,0.000000" ActionValue false)
    (if (not (Variables|Default|GetisUnturning))
      (Pawn|SetControlRotation (Pawn|GetController) (select (> ActionValue 0.0) (Math|Rotator|MakeRotator 0.0 0.0 0.0) (Math|Rotator|MakeRotator 0.0 0.0 1.8e+02))))))

(event Input|EnhancedActionEvents|EnhancedInputActionIA_Roll
  (params (ActionValue :type Boolean) (ElapsedSeconds :type Float%20%28double-precision%29) (TriggeredSeconds :type Float%20%28double-precision%29) (InputAction :type Input%20Action%20Object%20Reference :default "/Game/Input/Actions/IA_Roll.IA_Roll"))
  (bind _returnvalue (Transformation|GetActorForwardVector))
  (Utilities|FlowControl|DoOnce false :!label _label
    (:Completed
      (|RootMovement (Variables|Character|GetCharacterMovement) _returnvalue 5e+02 0.7 false "/Game/Blueprints/Curve/Curve_RollMovement.Curve_RollMovement" "MaintainLastRootMotionVelocity" _returnvalue 0.0 false
        (:then
          (Sprite|SetFlipbook (Variables|Default|GetSprite) "/Game/PaperAssets/Knight/FlipBooks/FB_Roll.FB_Roll")
          (Components|Timeline|SetLooping (Variables|Default|GetSprite) false)
          (Variables|Default|SetIsUnstopableAnimation true)
          (Variables|Default|SetisUnturning true)
          (Utilities|FlowControl|Delay 0.7)
          (goto _label Reset))))))

(event Input|EnhancedActionEvents|EnhancedInputActionIA_Attack
  (params (ActionValue :type Boolean) (ElapsedSeconds :type Float%20%28double-precision%29) (TriggeredSeconds :type Float%20%28double-precision%29) (InputAction :type Input%20Action%20Object%20Reference :default "/Game/Input/Actions/IA_Attack.IA_Attack"))
  (Sprite|SetFlipbook (Variables|Default|GetSprite) "/Game/PaperAssets/Knight/FlipBooks/FB_Attack_0.FB_Attack_0")
  (Components|Timeline|SetLooping (Variables|Default|GetSprite) false)
  (Variables|Default|SetIsUnstopableAnimation true)
  (Variables|Default|SetIsUnmovableAnimation true))

(event Input|EnhancedActionEvents|EnhancedInputActionIA_Attack_Second
  (params (ActionValue :type Boolean) (ElapsedSeconds :type Float%20%28double-precision%29) (TriggeredSeconds :type Float%20%28double-precision%29) (InputAction :type Input%20Action%20Object%20Reference :default "/Game/Input/Actions/IA_Attack_Second.IA_Attack_Second"))
  (Sprite|SetFlipbook (Variables|Default|GetSprite) "/Game/PaperAssets/Knight/FlipBooks/FB_Attack_1.FB_Attack_1")
  (Components|Timeline|SetLooping (Variables|Default|GetSprite) false)
  (Variables|Default|SetIsUnstopableAnimation true)
  (Variables|Default|SetIsUnmovableAnimation true))

(event Collision|EventActorBeginOverlap
  (params (OtherActor :type Actor%20Object%20Reference)))

(event EventTick
  (params (DeltaSeconds :type Float%20%28single-precision%29))
  (CallFunction|UpdateAnimationMoving)
  (CallFunction|HitCheck)
  (Development|PrintString (Utilities|String|ToString(Boolean) (Variables|Default|GetIsUnmovableAnimation))))

(event EventBeginPlay
  (bind _asplayer_controller (Utilities|Casting|CastToPlayerController (Pawn|GetController)))
  (Input|AddMappingContext (PlayerController|LocalPlayerSubsystems|GetEnhancedInputLocalPlayerSubsystem _asplayer_controller) "/Game/Input/IMC_Platformer.IMC_Platformer" 0 "(bIgnoreAllPressedKeysUntilRelease=True,bForceImmediately=False,bNotifyUserSettings=False)"))

(fn ConstructionScript)

(fn UpdateAnimationMoving
  (bind _returnvalue (Transformation|GetVelocity))
  (if (not (Variables|Default|GetIsUnstopableAnimation))
    (if (AI|Components|NavMovement|IsMovingonGround (Variables|Character|GetCharacterMovement))
      (if true
        (if (> (Math|Vector|VectorLength _returnvalue) 0.0)
          (if (== (Variables|Default|GetLastFrameFrowardDirection) (.Yaw (Math|Vector|GetYawPitchfromVector _returnvalue)))
            _
            (else
              _))
          (Components|Timeline|SetLooping (Variables|Default|GetSprite) true)
          (Sprite|SetFlipbook (Variables|Default|GetSprite) "/Game/PaperAssets/Knight/FlipBooks/FB_Run.FB_Run")
          (else
            (Sprite|SetFlipbook (Variables|Default|GetSprite) "/Game/PaperAssets/Knight/FlipBooks/FB_Idle.FB_Idle"))))
      (elif (> (.z (Transformation|GetVelocity)) 0.0)
        (Sprite|SetFlipbook (Variables|Default|GetSprite) "/Game/PaperAssets/Knight/FlipBooks/FB_Jump.FB_Jump")
        (else
          (Sprite|SetFlipbook (Variables|Default|GetSprite) "/Game/PaperAssets/Knight/FlipBooks/FB_Fall.FB_Fall"))))))

(fn RestartAnimation
  (Components|Timeline|SetLooping (Variables|Default|GetSprite) true)
  (if (not (Audio|Components|Audio|IsPlaying (Variables|Default|GetSprite)))
    (Audio|Components|Audio|Play (Variables|Default|GetSprite))
    (Variables|Default|SetIsUnstopableAnimation false)
    (Variables|Default|SetIsUnmovableAnimation false)
    (Variables|Default|SetisUnturning false)))

(fn HitCheck
  (for _array_element (Collision|GetOverlappingActors (Variables|Default|GetHitbox) 0 :!class /Script/Engine.PrimitiveComponent)
    (if (!= _array_element self)
      (Game|Damage|ApplyDamage _array_element (Variables|Default|GetDamageAmount) 0 0))))